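; Grid tile actor for the A* game that shows its ground type and hover, selection and path states.
; Cursor hover and click events set the tile's state and notify the owning grid, which stores each tile's data by grid index.
; SetTileColor drives material parameters from that data and state, brightening on hover and overriding with blue on a path.
; After a short BeginPlay delay, it scales the mesh to the grid's tile size and initializes its widget.
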(event OnBeginCursorOver(StaticMesh)
  (params (TouchedComponent :type Primitive%20Component%20Object%20Reference))
  (CallFunction|EventStartOverTile)
  (Default|EventNewTileOvered (Variables|GridTile|GetBP_Grid) self))

(event OnEndCursorOver(StaticMesh)
  (params (TouchedComponent :type Primitive%20Component%20Object%20Reference)))

(event OnClicked(StaticMesh)
  (params (TouchedComponent :type Primitive%20Component%20Object%20Reference) (ButtonPressed :type Key%20Structure))
  (CallFunction|EventSelectTile)
  (Default|EventNewTileSelected (Variables|GridTile|GetBP_Grid) self))

(event Custom|Event_DeselectTile
  (Variables|GridTile|SetbIsSelected false)
  (Grid|SetTileColor))

(event Custom|Event_SelectTile
  (Variables|GridTile|SetbIsSelected true)
  (Grid|SetTileColor))

(event Custom|Event_StartOverTile
  (Variables|GridTile|SetbIsOvered true)
  (Grid|SetTileColor))

(event Custom|Event_EndOverTile
  (Variables|GridTile|SetbIsOvered false)
  (Grid|SetTileColor))

(event Custom|Event_IsInPath
  (params (bIsInPath :type Boolean))
  (Variables|GridTile|SetbIsInPath bIsInPath)
  (Grid|SetTileColor))

(event EventBeginPlay
  (Utilities|FlowControl|Delay 0.2)
  (Grid|SetTileColor)
  (Grid|SetTileSize)
  (Grid|SetWidgetVariables))

(fn ConstructionScript)

(fn SetTileColor
  (Utilities|FlowControl|Sequence
    (:then_0
      (switch Utilities|FlowControl|Switch|SwitchonEnum_GroundType (.groundtype (Grid|GetTileData))
        (:NewEnumerator0
          (LocalVariables|SetTile%20Color "(R=0.703125,G=0.703125,B=0.703125,A=1.000000)"))
        (:NewEnumerator1
          (LocalVariables|SetTile%20Color "(R=0.287545,G=0.567708,B=0.109259,A=1.000000)"))
        (:NewEnumerator2
          (LocalVariables|SetTile%20Color "(R=0.255208,G=0.254560,B=0.130263,A=1.000000)"))
        (:NewEnumerator3
          (LocalVariables|SetTile%20Color "(R=0.307292,G=0.012804,B=0.012804,A=1.000000)"))
        (:NewEnumerator4
          (LocalVariables|SetTile%20Color "(R=0.713542,G=0.680731,B=0.676382,A=1.000000)"))))
    (:then_1
      (if (Variables|GridTile|GetbIsSelected)
        (Rendering|Material|SetScalarParameterValueonMaterials (Variables|Default|GetStaticMesh) "bIsSelected" 1.0)
        (else
          (Rendering|Material|SetScalarParameterValueonMaterials (Variables|Default|GetStaticMesh) "bIsSelected" 0.0))))
    (:then_2
      (if (Variables|GridTile|GetbIsOvered)
        (LocalVariables|SetTile%20Color (Math|Conversions|ToLinearColor(Vector) (* (Math|Conversions|ToVector(LinearColor) (LocalVariables|GetTile%20Color)) 3.0)))))
    (:then_3
      (if (Variables|GridTile|GetbIsInPath)
        (LocalVariables|SetTile%20Color "(R=0.066006,G=0.313562,B=0.651042,A=1.000000)")))
    (:then_4
      (Rendering|Material|SetVectorParameterValueonMaterials (Variables|Default|GetStaticMesh) "TileColor" (Math|Conversions|ToVector(LinearColor) (LocalVariables|GetTile%20Color))))))

(fn GetTileData
  (return (.Value (Utilities|Map|Find (Variables|/Game/AStarGame/Blueprints/Grid/BP_Grid.BP_Grid_C|GetStruct_Tiles (Variables|GridTile|GetBP_Grid)) (Variables|GridTile|GetGridIndex)))))

(fn SetTileSize
  (bind _bp_grid (Variables|GridTile|GetBP_Grid))
  (bind _staticmesh (Variables|Default|GetStaticMesh))
  (bind _returnvalue (Transformation|GetWorldScale _staticmesh))
  (bind _tilesize (Variables|/Game/AStarGame/Blueprints/Grid/BP_Grid.BP_Grid_C|GetTileSize _bp_grid))
  (bind _returnvalue_2 (/ _tilesize 5e+01))
  (bind _returnvalue_3 (* _returnvalue _returnvalue_2))
  (Transformation|SetWorldScale3D _staticmesh (Math|Vector|MakeVector (.x _returnvalue_3) (.y _returnvalue_3) 1.0)))

(fn SetWidgetVariables
  (bind _widget (Variables|Default|GetWidget))
  (bind _returnvalue (UserInterface|GetUserWidgetObject _widget))
  (bind _aswbp_grid_tile (Utilities|Casting|CastToWBP_GridTile _returnvalue))
  (Variables|/Game/AStarGame/Blueprints/Grid/WBP_GridTile.WBP_GridTile_C|SetGrid _aswbp_grid_tile (Variables|GridTile|GetBP_Grid))
  (Variables|/Game/AStarGame/Blueprints/Grid/WBP_GridTile.WBP_GridTile_C|SetGridIndex _aswbp_grid_tile (Variables|GridTile|GetGridIndex)))